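; BP_Ball is a player-controlled physics ball that rolls and jumps.
; Forward/Backward and Left/Right axis inputs feed a shared torque node on SMBall, scaled by AccellerationFactor.
; Jump applies an upward impulse as a velocity change, gated by a CanJump flag that any hit re-arms, without checking for ground.
; Sounds play on jump and on the first hit afterward.
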(event `InputAxis|Forward/Backward`
  (params (AxisValue :type "Float (single-precision)"))
  ;[1 1 1] Movement
  (`PrimitiveComponent.AddTorqueInRadians` (`self.SM_Ball`) (`KismetMathLibrary.MakeVector` (* (`self.AccellerationFactor`) (stale `InputAxis|Left/Right` AxisValue)) (* AxisValue (`self.AccellerationFactor`))) "None" true :!label _label))

(event `InputAxis|Left/Right`
  (params (AxisValue :type "Float (single-precision)"))
  ;[1 1 1] Movement
  (goto _label))

(event `InputAction|Jump`
  (params (Key :type "Key Structure"))
  ;[1 1 1] Jump and Play Sound
  (:`Pressed`
    (if (`self.CanJump`)
      (`PrimitiveComponent.AddImpulse` (`self.SM_Ball`) (`KismetMathLibrary.MakeVector` 0.0 0.0 (`self.Impulse`)) "None" true)
      (set `self.CanJump` false)
      (`GameplayStatics.PlaySound2D` "/Engine/VREditor/Sounds/UI/Laser_Push.Laser_Push" 1.0 1.0 0.0 null null))))

(event `self.ReceiveHit`
  (params (MyComp :type "PrimitiveComponent Object Reference") (Other :type "Actor Object Reference") (OtherComp :type "PrimitiveComponent Object Reference") (bSelfMoved :type Boolean) (HitLocation :type "Vector Structure") (HitNormal :type "Vector Structure") (NormalImpulse :type "Vector Structure") (Hit :type "HitResult Structure (by ref)"))
  ;[1 1 1] If on ground, set CanJump to True. If CanJump is False play sound on jump.
  (if (not (`self.CanJump`))
    (`GameplayStatics.PlaySound2D` "/Engine/VREditor/Sounds/UI/Laser_Pull.Laser_Pull" 1.0 1.0 0.0 null null))
  (set `self.CanJump` true))

(fn `UserConstructionScript`)